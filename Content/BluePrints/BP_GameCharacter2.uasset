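; Player character Blueprint that aims and throws pickable rocks while it has any left.
; The first AimThrowObject press starts aiming; the next plays the throw animation, spends a rock and launches a spawned physics rock away from the character through the throw reference point.
; While aiming, Tick rebuilds a predicted trajectory from spline meshes, destroying the previous ones each frame.
; Tick also prints a debug message when IsVisibleInLight is set.
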(event `self.ReceiveTick`
  (params (DeltaSeconds :type "Float (single-precision)"))
  (bind _splinecomponent (`self.SplineComponent`))
  (bind _returnvalue (`SceneComponent.K2_GetComponentLocation` (`self.ThrowableReferenceComponent`)))
  (`SplineComponent.ClearSplinePoints` (`self.SplineComponent`) true)
  (for _array_element (`self.SplineMeshComponents`)
    (`ActorComponent.K2_DestroyComponent` _array_element))
  (`KismetArrayLibrary.Array_Clear` (`self.SplineMeshComponents`))
  (if (`self.bIsAiming`)
    (bind _predictresult (`GameplayStatics.Blueprint_PredictProjectilePath_Advanced` (make `PredictProjectilePathParams` _returnvalue (* (`KismetMathLibrary.GetDirectionUnitVector` (`self.K2_GetActorLocation`) _returnvalue) (`self.ThrowForce`)) false 0.0 3.0 true "ECC_WorldStatic" _ (`|MakeArray` self :!type "Actor Object Reference"))))
    (for (_array_element_2 _array_index) (break `PredictProjectilePathResult` _predictresult)
      (`SplineComponent.AddSplinePointAtIndex` (`self.SplineComponent`) (`.Location` (break `PredictProjectilePathPointData` _array_element_2)) _array_index "Local" true))
    (for _index (range (+ (- (`SplineComponent.GetNumberOfSplinePoints` (`self.SplineComponent`)) 2) 1))
      (bind _returnvalue_2 (`AddComponent|NODE_AddSplineMeshComponent-2` :`bManualAttachment` true))
      (bind _returnvalue_3 (+ _index 1))
      (`SplineMeshComponent.SetStartAndEnd` _returnvalue_2 (`SplineComponent.GetLocationAtSplinePoint` _splinecomponent _index "Local") (`SplineComponent.GetTangentAtSplinePoint` _splinecomponent _index "Local") (`SplineComponent.GetLocationAtSplinePoint` _splinecomponent _returnvalue_3 "Local") (`SplineComponent.GetTangentAtSplinePoint` _splinecomponent _returnvalue_3 "Local") true)
      (`KismetArrayLibrary.Array_Add` (`self.SplineMeshComponents`) _returnvalue_2)))
  (if (`self.bIsVisibleInLight`)
    (`KismetSystemLibrary.PrintString` "Is visible in light"))
  (if true
    _))

(event `self.AimThrowObject`
  (bind _mesh (`self.Mesh`))
  (if (> (`self.RockAmount`) 0)
    (if (`self.bIsAiming`)
      (`SkeletalMeshComponent.PlayAnimation` _mesh "/Game/Characters/Animations/Throw_Object_Anim_mixamo_com.Throw_Object_Anim_mixamo_com" false)
      (bind _returnvalue (`self.GetRockAmount`))
      (bind _result (`/Engine/EditorBlueprintResources/StandardMacros.DecrementInt` _returnvalue)
        (:`  `
          (`self.SetRockAmount` _result)
          (set `self.bIsAiming` false)
          (`KismetSystemLibrary.Delay` 0.7)
          (bind _returnvalue_2 (`|SpawnActorFromClass` "/Game/BluePrints/WorldActors/BP_PickableRock1.BP_PickableRock1_C" (`KismetMathLibrary.MakeTransform` (`SceneComponent.K2_GetComponentLocation` (`self.ThrowableReferenceComponent`)) (`self.K2_GetActorRotation`) (0.2 0.2 0.2)) "Undefined" "OverrideRootScale" null null))
          (`PrimitiveComponent.SetSimulatePhysics` (`/Game/BluePrints/WorldActors/BP_PickableRock1.StaticMesh` _returnvalue_2) true)
          (`PrimitiveComponent.SetPhysicsLinearVelocity` (`/Game/BluePrints/WorldActors/BP_PickableRock1.StaticMesh` _returnvalue_2) (* (`KismetMathLibrary.GetDirectionUnitVector` (`self.K2_GetActorLocation`) (`self.K2_GetActorLocation` _returnvalue_2)) (`self.ThrowForce`)) false "None")
          (set `/Game/BluePrints/WorldActors/BP_PickableRock1.bIsThrown` true _returnvalue_2)
          (`KismetSystemLibrary.Delay` 2.0)
          (`SkeletalMeshComponent.SetAnimationMode` _mesh "AnimationBlueprint")))
      (else
        ;[1 1 1] Continuation in predict projectile path
        (set `self.bIsAiming` true)))))

(fn `UserConstructionScript`)