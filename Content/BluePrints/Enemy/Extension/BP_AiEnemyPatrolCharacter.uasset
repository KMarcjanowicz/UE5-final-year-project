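; BP_AiEnemyPatrolCharacter is an AI patrol enemy character Blueprint that keeps its state and alarmed labels facing the player's view.
; Each Tick calls the parent Tick, then rotates both label components in world space toward player 0's camera manager.
; The look-at rotation starts from the actor's location rather than each label's, so both labels share the same billboard orientation.
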(event `self.ReceiveTick`
  (params (DeltaSeconds :type "Float (single-precision)"))
  (`parent.ReceiveTick` DeltaSeconds)
  (`SceneComponent.K2_SetWorldRotation` (`self.StateLabelComp`) (`KismetMathLibrary.FindLookAtRotation` (`self.K2_GetActorLocation`) (`self.K2_GetActorLocation` (`GameplayStatics.GetPlayerCameraManager` 0))) false false)
  (`SceneComponent.K2_SetWorldRotation` (`self.AlarmedLabelComp`) (`KismetMathLibrary.FindLookAtRotation` (`self.K2_GetActorLocation`) (`self.K2_GetActorLocation` (`GameplayStatics.GetPlayerCameraManager` 0))) false false))

(fn `UserConstructionScript`)