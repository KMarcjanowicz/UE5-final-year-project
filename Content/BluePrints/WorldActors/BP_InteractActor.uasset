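; BP_InteractActor is a world actor that highlights itself when the player can interact with it.
; On BeginPlay it caches the player's GameCharacter, then overlap events from that player toggle IsPickable and the "Selected" scalar parameter on SMMesh's materials.
; Interact is a placeholder that prints a debug string and returns true without checking IsPickable.
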(event `self.ReceiveBeginPlay`
  (bind _asgame_character (cast `GameCharacter` (`GameplayStatics.GetPlayerPawn` 0)))
  (set `self.Player` _asgame_character))

(event `self.ReceiveActorBeginOverlap`
  (params (OtherActor :type "Actor Object Reference"))
  (if (== OtherActor (`self.Player`))
    (`MeshComponent.SetScalarParameterValueOnMaterials` (`self.SM_Mesh`) "Selected" 1.0)
    (set `self.bIsPickable` true)))

(event `self.ReceiveActorEndOverlap`
  (params (OtherActor :type "Actor Object Reference"))
  (if (== OtherActor (`self.Player`))
    (`MeshComponent.SetScalarParameterValueOnMaterials` (`self.SM_Mesh`) "Selected" 0.0)
    (set `self.bIsPickable` false)))

(fn `Interact`
  (params (_Interactor :type "Character Object Reference"))
  (returns (`_bDidInteract?` :type Boolean))
  (`KismetSystemLibrary.PrintString` "Interacted")
  (return true))

(fn `UserConstructionScript`)