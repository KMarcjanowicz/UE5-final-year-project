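; Swinging door actor that opens and closes through Interact, which AI-tagged pawns trigger automatically on overlap.
; A timeline rotates the Arrow component's yaw, with play rate set from open or close durations, and toggles IsOpen when finished.
; Front and back trigger volumes choose the swing direction while the door is closed, gated by an IsInUse flag from actor overlap.
; Player overlap toggles a "Selected" material highlight on the door mesh.
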(event `self.ReceiveBeginPlay`
  (bind _asgame_character (cast `GameCharacter` (`GameplayStatics.GetPlayerPawn` 0)))
  (set `self.Player` _asgame_character))

(event `Door Open`
  (`KismetSystemLibrary.PrintString` "Open Door")
  (bind (_direction _door_open_close) (`Timeline|Door Movement` :!label _label)
    (:`Update`
      (`SceneComponent.K2_SetRelativeRotation` (`self.Arrow`) (`KismetMathLibrary.MakeRotator` 0.0 0.0 (`KismetMathLibrary.Lerp` (`self.Closed Position`) (`self.Opened Position`) _door_open_close)) false false))
    (:`Finished`
      (set `self.bIsOpen` (not (`self.bIsOpen`))))))

(event `Door Close`
  (`KismetSystemLibrary.PrintString` "Close Door")
  (goto _label :!via `Reverse`))

(event `self.ReceiveActorBeginOverlap`
  (params (OtherActor :type "Actor Object Reference"))
  (if (== OtherActor (`self.Player`))
    (`MeshComponent.SetScalarParameterValueOnMaterials` (`self.SM_Door`) "Selected" 1.0))
  (set `self.bIsInUse` true))

(event `self.ReceiveActorEndOverlap`
  (params (OtherActor :type "Actor Object Reference"))
  (if (== OtherActor (`self.Player`))
    (`MeshComponent.SetScalarParameterValueOnMaterials` (`self.SM_Door`) "Selected" 0.0))
  (set `self.bIsInUse` false))

(event `self.Open Door REF Front.OnComponentBeginOverlap`
  (params (OverlappedComponent :type "PrimitiveComponent Object Reference") (OtherActor :type "Actor Object Reference") (OtherComp :type "PrimitiveComponent Object Reference") (OtherBodyIndex :type Integer) (bFromSweep :type Boolean) (SweepResult :type "HitResult Structure (by ref)"))
  (if (!= OtherActor "BP_Door")
    (`KismetSystemLibrary.PrintString` "Front")
    (if (`self.bIsInUse`)
      (if (not (`self.bIsOpen`))
        (set `self.Opened Position` -90.0))
      (set `self.bIsInUse` false)
      (for _array_element (`Actor.Tags` OtherActor)
        (if (== _array_element "AIPawn")
          (`/Game/BluePrints/Interfaces/BPI_Interact.Interact` null))))))

(event `self.Open Door REF Back.OnComponentBeginOverlap`
  (params (OverlappedComponent :type "PrimitiveComponent Object Reference") (OtherActor :type "Actor Object Reference") (OtherComp :type "PrimitiveComponent Object Reference") (OtherBodyIndex :type Integer) (bFromSweep :type Boolean) (SweepResult :type "HitResult Structure (by ref)"))
  (if (!= OtherActor "BP_Door")
    (`KismetSystemLibrary.PrintString` "Back")
    (if (`self.bIsInUse`)
      (if (not (`self.bIsOpen`))
        (set `self.Opened Position` 90.0))
      (set `self.bIsInUse` false)
      (for _array_element (`Actor.Tags` OtherActor)
        (if (== _array_element "AIPawn")
          (`/Game/BluePrints/Interfaces/BPI_Interact.Interact` null))))))

(fn `Interact`
  (params (_Interactor :type "Character Object Reference"))
  (returns (`_bDidInteract?` :type Boolean))
  (if (not (`self.bIsOpen`))
    (`TimelineComponent.SetPlayRate` (`self.Door Movement`) (/ 1.0 (`self.Time to Open (s)`)))
    (`self.Door Open`)
    (else
      (`TimelineComponent.SetPlayRate` (`self.Door Movement`) (/ 1.0 (`self.Time to Close (s)`)))
      (`self.Door Close`)))
  (return true))

(fn `UserConstructionScript`)