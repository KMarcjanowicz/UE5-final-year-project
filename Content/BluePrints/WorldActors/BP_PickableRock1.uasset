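; BP_PickableRock1 is a rock actor that the player collects by touch and that acts as a noise source when thrown.
; Touching it while pickable increments the player's rock count, plays a pickup animation, then destroys the rock and restores Animation Blueprint mode.
; When thrown, its mesh hitting anything not of the player pawn's class plays a sound, reports a noise event, and destroys it after a short delay.
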(event `self.ReceiveHit`
  (params (MyComp :type "PrimitiveComponent Object Reference") (Other :type "Actor Object Reference") (OtherComp :type "PrimitiveComponent Object Reference") (bSelfMoved :type Boolean) (HitLocation :type "Vector Structure") (HitNormal :type "Vector Structure") (NormalImpulse :type "Vector Structure") (Hit :type "HitResult Structure (by ref)"))
  (bind _returnvalue (`self.K2_GetActorLocation`))
  (if (== MyComp (`self.StaticMesh`))
    (if (`self.bIsThrown`)
      (if (not (== (`GameplayStatics.GetObjectClass` Other) (`GameplayStatics.GetObjectClass` (`GameplayStatics.GetPlayerPawn` 0))))
        (`KismetSystemLibrary.PrintString` "Hit")
        (`GameplayStatics.PlaySoundAtLocation` "/Engine/VREditor/Sounds/UI/Camera_Shutter.Camera_Shutter" _returnvalue (struct) 1.0 1.0 0.0 null null null null)
        (`AISense_Hearing.ReportNoiseEvent` _returnvalue 1.0 self)
        (set `self.bIsThrown` false)
        (`KismetSystemLibrary.Delay` 0.2)
        (`self.K2_DestroyActor`)))))

(event `self.ReceiveActorOnInputTouchBegin`
  (params (FingerIndex :type "ETouchIndex Enum" :default "Touch1"))
  (bind _player (`self.Player`))
  (bind _mesh (`Character.Mesh` _player))
  (if (`self.bIsPickable`)
    (bind _returnvalue (`GameCharacter.GetRockAmount` _player))
    (bind _result (`/Engine/EditorBlueprintResources/StandardMacros.IncrementInt` _returnvalue)
      (:`  `
        (`GameCharacter.SetRockAmount` _player _result)
        (`SkeletalMeshComponent.PlayAnimation` _mesh "/Game/Characters/Animations/Pick-Up_Object_Anim_mixamo_com.Pick-Up_Object_Anim_mixamo_com" false)
        (`KismetSystemLibrary.Delay` 1.0)
        (`self.K2_DestroyActor`)
        (`SkeletalMeshComponent.SetAnimationMode` _mesh "AnimationBlueprint")))))

(fn `UserConstructionScript`)