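; BP_Treasure is a world pickup actor that awards score when touched through touch input while IsPickable is true.
; It passes its Score, fixed at 50 in the construction script, to BP_GameMode's SetScore and plays a pickup animation on the Player mesh.
; After a one-second delay it destroys itself, then switches the mesh back to Animation Blueprint mode.
; Nothing in this graph sets IsPickable or Player.
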(event `self.ReceiveActorOnInputTouchBegin`
  (params (FingerIndex :type "ETouchIndex Enum" :default "Touch1"))
  (bind _mesh (`Character.Mesh` (`self.Player`)))
  (if (`self.bIsPickable`)
    (bind _asbp_game_mode (cast `/Game/BluePrints/BP_GameMode` (`GameplayStatics.GetGameMode`)))
    (`GameGameMode.SetScore` _asbp_game_mode (`self.Score`))
    (`SkeletalMeshComponent.PlayAnimation` _mesh "/Game/Characters/Animations/Pick-Up_Object_Anim_mixamo_com.Pick-Up_Object_Anim_mixamo_com" false)
    (`KismetSystemLibrary.Delay` 1.0)
    (`self.K2_DestroyActor`)
    (`SkeletalMeshComponent.SetAnimationMode` _mesh "AnimationBlueprint")))

(fn `UserConstructionScript`
  (`parent.UserConstructionScript`)
  (set `self.Score` 50))