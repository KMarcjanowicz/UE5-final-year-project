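; BP_Puddle is a world puddle that plays footstep splashes and alerts AI hearing when the player moves quickly through it.
; Tick checks player overlap and, while no splash is stored, spawns a footstep sound with speed-scaled volume.
; Above a speed threshold, it stores that sound and reports speed-scaled noise, then stops and clears it after a short delay, throttling repeats.
; Below the threshold, sounds spawn every tick untracked.
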(event `self.ReceiveTick`
  (params (DeltaSeconds :type "Float (single-precision)"))
  (bind _returnvalue (`self.K2_GetActorLocation` (`GameplayStatics.GetPlayerCharacter` 0)))
  (bind _returnvalue_2 (`KismetMathLibrary.VSize` (`self.GetVelocity` (`GameplayStatics.GetPlayerCharacter` 0))))
  (bind _returnvalue_3 (`KismetMathLibrary.NormalizeToRange` _returnvalue_2 200.0 600.0))
  (if (`self.IsOverlappingActor` (`GameplayStatics.GetPlayerPawn` 0))
    (`self.Splash Sound`
      (:`then`)
      (:`else`
        (bind _returnvalue_4 (`GameplayStatics.SpawnSoundAtLocation` "/Game/Assets/Sounds/Footsteps/C_Puddle_Footstep.C_Puddle_Footstep" _returnvalue (struct) _returnvalue_3 1.0 0.0 null null))
        (if (> _returnvalue_2 300.0)
          (set `self.Splash Sound` _returnvalue_4)
          (`AISense_Hearing.ReportNoiseEvent` _returnvalue _returnvalue_3 (`GameplayStatics.GetPlayerCharacter` 0))
          (`KismetSystemLibrary.Delay` 0.5)
          (`AudioComponent.Stop` (`self.Splash Sound`))
          (set `self.Splash Sound` null))))))

(fn `UserConstructionScript`)